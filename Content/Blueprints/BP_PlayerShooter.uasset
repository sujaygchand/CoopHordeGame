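; Player shooter Blueprint that sets up the local player's HUD and shows health-change feedback.
; On BeginPlay, if locally controlled, it creates crosshair, ammo and health indicator widgets, stores them in UIWidgets and adds them to the viewport.
; The SHealth component's OnHealthChanged event draws the health delta as red debug text at the actor's location.
; A locally controlled health print is left unconnected.
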(event OnHealthChanged(SHealth)
  (params (HealthComp :type S%20Health%20Component%20Object%20Reference) (Health :type Float%20%28single-precision%29) (HealthDelta :type Float%20%28single-precision%29) (DamageType :type Damage%20Type%20Object%20Reference) (InstigatedBy :type Controller%20Object%20Reference) (DamageCauser :type Actor%20Object%20Reference))
  (Rendering|Debug|DrawDebugString (Transformation|GetActorLocation) (Utilities|String|ToString(Float) HealthDelta) 0 "(R=1.000000,G=0.000000,B=0.000000,A=1.000000)" 1.0))

(event EventBeginPlay
  ;[1 1 1] On Play
  (if (Pawn|IsLocallyControlled)
    (CallFunction|CreateWidgets)
    (CallFunction|AddWidgetstoViewport (Variables|Default|GetUIWidgets))))

(fn ConstructionScript)

(fn CreateWidgets
  ;[1 1 1] Creates Widgets
  (Utilities|Array|Clear (Variables|Default|GetUIWidgets))
  (bind _returnvalue (UserInterface|CreateWidget "/Game/UI/UMG_Crosshair.UMG_Crosshair_C"))
  (bind _output_get (Variables|Default|SetCrosshair%20UI _returnvalue))
  (Utilities|Array|Add (Variables|Default|GetUIWidgets) _output_get)
  (bind _returnvalue_2 (UserInterface|CreateWidget "/Game/UI/UMG_Ammo.UMG_Ammo_C"))
  (bind _output_get_2 (Variables|Default|SetAmmo%20UI _returnvalue_2))
  (Utilities|Array|Add (Variables|Default|GetUIWidgets) _output_get_2)
  (bind _returnvalue_3 (UserInterface|CreateWidget "/Game/UI/UMG_HealthIndicator.UMG_HealthIndicator_C"))
  (bind _output_get_3 (Variables|Default|SetHealthUI _returnvalue_3))
  (Utilities|Array|Add (Variables|Default|GetUIWidgets) _output_get_3))

(fn AddWidgetstoViewport
  (params (Widgets :type Array%20of%20User%20Widget%20Object%20References))
  (for _array_element Widgets
    (UserInterface|Viewport|AddtoViewport _array_element 0))
  (return))