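; Super speed powerup that temporarily doubles the walk speed of the actor it is activated on.
; BeginPlay caches the base MaxWalkSpeed from the first player's pawn, not from the powered-up actor.
; OnActivated stores the actor and applies the multiplied speed through its CharacterMovementComponent.
; OnExpired restores the cached speed and calls the parent's expiry only if that component is valid, with both events printing the new speed.
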(event EventBeginPlay
  ;[1 1 1] On Play
  (Variables|Default|SetBaseSpeed (Variables|/Script/Engine.CharacterMovementComponent|GetMaxWalkSpeed (Actor|GetComponentbyClass (Game|Player|GetPlayerPawn 0) "/Script/Engine.CharacterMovementComponent"))))

(event EventOnActivated
  (params (CurrentActor :type Actor%20Object%20Reference))
  ;[1 1 1] On Activated
  (bind _output_get (Variables|Default|SetActorPoweredUp CurrentActor))
  (Utilities|IsValid (Actor|GetComponentbyClass _output_get "/Script/Engine.CharacterMovementComponent")
    (:Is%20Valid
      (bind _output_get_2 (Variables|/Script/Engine.CharacterMovementComponent|SetMaxWalkSpeed (Actor|GetComponentbyClass _output_get "/Script/Engine.CharacterMovementComponent") (* (Variables|Default|GetBaseSpeed) 2.0)))
      (Development|PrintString (Utilities|String|ToString(Float) _output_get_2)))))

(event EventOnExpired
  (bind _actorpoweredup (Variables|Default|GetActorPoweredUp))
  (bind _returnvalue (Actor|GetComponentbyClass _actorpoweredup "/Script/Engine.CharacterMovementComponent"))
  ;[1 1 1] On Expired
  (Utilities|IsValid _returnvalue
    (:Is%20Valid
      (bind _output_get (Variables|/Script/Engine.CharacterMovementComponent|SetMaxWalkSpeed _returnvalue (Variables|Default|GetBaseSpeed)))
      (Development|PrintString (Utilities|String|ToString(Float) _output_get))
      (|CallParentFunction))))

(fn ConstructionScript)